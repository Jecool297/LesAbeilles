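; Test Blueprint for a Paper2D character sprite that moves to a clicked location with a directional flipbook.
; ClickLocation, ignored while moving, compares the click direction's dot products against the sprite's forward and up vectors to pick Up, Down, Left or Right, printing debug values.
; MoveComponentTo eases it to a target computed in player-pawn space, then resets to Down.
; Disconnected leftovers include a line trace and a looping square-patrol timeline chain.
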(event EventBeginPlay)

(event EventTick
  (params (DeltaSeconds :type Float%20%28single-precision%29)))

(event EventClickLocation
  (params (NewParam :type Vector :default "0, 0, 0"))
  (bind _returnvalue (Game|Player|GetPlayerPawn 0))
  (bind _paperflipbook (Variables|Default|GetPaperFlipbook))
  (bind _paperflipbook_2 (Variables|Default|GetPaperFlipbook))
  (bind _paperflipbook_3 (Variables|Default|GetPaperFlipbook))
  (bind _returnvalue_2 (Transformation|GetActorTransform _returnvalue))
  (bind _returnvalue_3 (Math|Transform|InverseTransformLocation _returnvalue_2 NewParam))
  (bind (_x _y) (Math|Vector|BreakVector _returnvalue_3))
  (if (not (Variables|Default|GetIsMoving))
    (Variables|Default|SetIsMoving true)
    (bind _output_get (Variables|Default|SetOrientation (Math|Vector|Normalize (- NewParam (Transformation|GetWorldLocation (Variables|Default|GetPaperFlipbook))))))
    (Development|PrintString (Utilities|String|ToString(Boolean) (> (Math|Vector|DotProduct (Math|Vector|GetForwardVector _paperflipbook_2) _output_get) (Math|Vector|DotProduct _output_get (Math|Vector|GetUpVector _paperflipbook_2)))))
    (Development|PrintString (Utilities|String|ToString(Float) (Math|Vector|DotProduct (Math|Vector|GetForwardVector _paperflipbook_2) _output_get)) true true "(R=1.000000,G=0.737253,B=0.000000,A=1.000000)")
    (Sprite|SetFlipbook _paperflipbook (select (> (Math|Vector|DotProduct (Math|Vector|GetForwardVector _paperflipbook_2) _output_get) (Math|Vector|DotProduct _output_get (Math|Vector|GetUpVector _paperflipbook_2))) (select (> (Math|Vector|DotProduct (Math|Vector|GetForwardVector _paperflipbook_2) _output_get) 0.0) "/Game/Art/Personnages/FlipBook/Down.Down" "/Game/Art/Personnages/FlipBook/Up.Up") (select (> (Math|Vector|DotProduct (Math|Vector|GetForwardVector _paperflipbook_2) _output_get) 0.0) "/Game/Art/Personnages/FlipBook/Right.Right" "/Game/Art/Personnages/FlipBook/Left.Left")))
    (Components|MoveComponentTo _paperflipbook_3 (Math|Vector|MakeVector 0.0 (* _y -1.0) _x) (Variables|/Script/Engine.SceneComponent|GetRelativeRotation _paperflipbook_3) true false 1.0 false)
    (Variables|Default|SetIsMoving false)
    (Sprite|SetFlipbook _paperflipbook "/Game/Art/Personnages/FlipBook/Down.Down")))

(fn ConstructionScript)

(fn NewFunction)