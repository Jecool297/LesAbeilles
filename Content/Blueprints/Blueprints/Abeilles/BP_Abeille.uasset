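; Selectable bee piece that moves between honeycomb cells (BP_Alveole) within a range set by its bee type.
; The construction script reads the type's data table row to set a dynamic material texture, health and movement distance.
; A sphere overlap of that radius drives cell accessibility updates, validates moves to available cells and detects other bees as attack opportunities.
; Moving requires selection and clears it on success.
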(event EventBeginPlay)

(event Collision|EventActorBeginOverlap
  (params (OtherActor :type Actor%20Object%20Reference)))

(event EventTick
  (params (DeltaSeconds :type Float%20%28single-precision%29)))

(event EventSelectionne
  (CallFunction|PrintMessage true (Utilities|String|Append (Utilities|GetDisplayName self) (Utilities|String|EnumtoString (Variables|01-SetupAlveole|GetTypeAbeille))) "   Is Selected" "(R=1.000000,G=0.012416,B=0.000000,A=1.000000)" 5.0)
  (Variables|Default|SetIsSelected? true)
  (bind _outactors (Actor|GetAllActorsOfClass "/Game/Blueprints/Blueprints/Alveoles/BP_Alveole.BP_Alveole_C"))
  (for _array_element _outactors
    (Class|BPI|CheckAccessibilite(Message) _array_element false)))

(event EventDeplacementAbeille
  (params (AlveoleActor :type Actor%20Object%20Reference))
  ;[0.15 0.15 0.15 0.5] Si l'abeille est sélectionné, elle peut-être joué
  (if (Variables|Default|GetIsSelected?)
    ;[0.15 0.15 0.15 0.5] Vérifie si l'aveole cliqué est a porté pour le déplacement
    (bind _actordanslazone (CallFunction|ActorProche "/Game/Blueprints/Blueprints/Alveoles/BP_Alveole.BP_Alveole_C"))
    (for _array_element _actordanslazone
      (bind _asbp_alveole (Utilities|Casting|CastToBP_Alveole _array_element))
      (Class|BPI|CheckAccessibilite(Message) _array_element false)
      (if (and (== _array_element AlveoleActor) (Variables|/Game/Blueprints/Blueprints/Alveoles/BP_Alveole.BP_Alveole_C|GetEstDisponible? _asbp_alveole))
        ;[0.15 0.15 0.15 0.5] Déplace l'abeille à l'aveole correspondante
        (Transformation|SetActorLocation (+ (Transformation|GetActorLocation AlveoleActor) "0.000000,0.000000,10.000000") false false)
        (Variables|Default|SetIsSelected? false)
        (else
          (CallFunction|PrintMessage true "" "Alveole Hors de portée ou indisponible" "(R=1.000000,G=0.012416,B=0.000000,A=1.000000)" 5.0))))))

(event EventCheckAccessibilite
  (params (Accessible? :type Boolean))
  (bind _outactors (Actor|GetAllActorsOfClass "/Game/Blueprints/Blueprints/Alveoles/BP_Alveole.BP_Alveole_C"))
  (for _array_element _outactors
    (Class|BPI|CheckAccessibilite(Message) _array_element false))
  (bind _actordanslazone (CallFunction|ActorProche "/Game/Blueprints/Blueprints/Alveoles/BP_Alveole.BP_Alveole_C"))
  (for _array_element_2 _actordanslazone
    (Class|BPI|CheckAccessibilite(Message) _array_element_2 true)))

(fn ConstructionScript
  (bind _datatable (Variables|Default|GetDataTable))
  ;[0.15 0.15 0.15 0.5] Vérifie et stock les information de l'abeille sélectionné
  (bind _outrownames (DataTable|GetDataTableRowNames _datatable))
  (bind _returnvalue (Class|DataTableFunctionLibrary|DoesDataTableRowExist _datatable (Utilities|Array|Get(acopy) _outrownames (Math|Conversions|ToInteger(Byte) (Variables|01-SetupAlveole|GetTypeAbeille)))))
  (if _returnvalue
    (bind _returnvalue_2 (Utilities|GetDataTableRow _datatable (Utilities|Array|Get(acopy) _outrownames (Math|Conversions|ToInteger(Byte) (Variables|01-SetupAlveole|GetTypeAbeille))))
      (:then
        (Variables|Default|SetStructureAbeille _returnvalue_2)
        ;[0.15 0.15 0.15 0.5] Instance le materiel Master Instance d'alvéole
        (bind _returnvalue_3 (Rendering|Material|CreateDynamicMaterialInstance (Variables|Materials|GetMasterMaterialAbeille) "None" "None" :!class /Script/Engine.KismetMaterialLibrary))
        (Variables|Materials|SetMateriaInstAbeille _returnvalue_3)
        (CallFunction|ChangementTextureAbeille)
        (CallFunction|SetupInitial)))))

(fn ChangementTextureAbeille
  (bind _materiainstabeille (Variables|Materials|GetMateriaInstAbeille))
  (bind _structureabeille (Variables|Default|GetStructureAbeille))
  (bind _imageabeille (Utilities|Struct|BreakStruct_Abeille _structureabeille))
  ;[0.15 0.15 0.15 0.5] Applique la texture correspondante à l'alvéole choisi
  (Rendering|Material|SetTextureParameterValue _materiainstabeille "Diffuse" _imageabeille)
  (Rendering|Material|SetTextureParameterValue _materiainstabeille "OpacityMask" _imageabeille)
  ;[0.15 0.15 0.15 0.5] Applique le materiel après le changement de texture
  (Rendering|Material|SetMaterial (Variables|Default|GetAbeille) 0 (Variables|Materials|GetMateriaInstAbeille)))

(fn SetupInitial
  (bind _structureabeille (Variables|Default|GetStructureAbeille))
  (bind (_nom _typeabeille _pointdevie _distancedeplacement) (Utilities|Struct|BreakStruct_Abeille _structureabeille))
  (bind _output_get (Variables|Vie|SetVieMax _pointdevie))
  (Variables|Vie|SetVieActuelle _output_get)
  (Variables|Default|SetDistance%20Deplacement (* _distancedeplacement 256)))

(fn ActorProche
  (params (FiltreActor :type Object%20Class%20Reference))
  ;[0.15 0.15 0.15 0.5] Effectue une zone des alveoles à porté selon  le type d'abeille
  (bind (_outactors _returnvalue) (Collision|SphereOverlapActors (Transformation|GetActorLocation) (Math|Conversions|ToFloat(Integer) (Variables|Default|GetDistance%20Deplacement)) (Utilities|Array|MakeArray "ObjectTypeQuery1" "ObjectTypeQuery2") FiltreActor (Utilities|Array|MakeArray self)))
  (CallFunction|PrintMessage true "" (Utilities|GetDisplayName (Utilities|Array|Get(acopy) _outactors)) "(R=1.000000,G=0.515661,B=0.000000,A=1.000000)" 1e+01)
  (return _outactors _returnvalue))

(fn CheckOpportuniteAttaque
  (bind _actordetecte (CallFunction|ActorProche "BP_Abeille_C"))
  (return _actordetecte))

(fn GetAbeilleInfos
  (return (Variables|Default|GetStructureAbeille)))

(fn GetAlveoleInfos
  (return "NewEnumerator0"))