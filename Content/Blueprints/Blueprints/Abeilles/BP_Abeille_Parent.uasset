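; Parent Blueprint for bees that are selected, moved between honeycomb cells (alvéoles) and destroyed when attacked.
; Construction reads stats and texture from a DataTable row indexed by bee type, applying them through a dynamic material.
; A sphere overlap scaled by move distance finds cells in range, whose availability is set via BPI_Alveole messages.
; Selection and moves reset cells, then call CheckSurroundings, left empty here; CanPond always returns false.
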(event EventResetUnRecheableSpaces
  (Utilities|SetsSpacesUnavailable))

(event EventCheckSurroundings)

(event EventIsBeingAttacked
  (Actor|DestroyActor))

(event EventBeeSelected?
  (params (IsSelected :type Boolean))
  ;[0.15 0.15 0.15 0.5] Gère l'état de l'abeille une fois sélectionné
  ;;[0.15 0.09822 0 0.5] Débug du type d'abeille sélectionné avec son nom  d'actor
  (Variables|Default|SetIsSelected? IsSelected)
  (CallFunction|PrintMessage true "BP_Abeille_Parent::  " (Utilities|String|Append (Utilities|GetDisplayName self) (Utilities|String|EnumtoString (Variables|01-SetupAlveole|GetTypeAbeille)) "   Is Selected") "(R=0.157585,G=1.000000,B=0.000000,A=1.000000)" 5.0)
  ;;[0.15 0.15 0.15 0.5] Réinitialise les mouvements qui étaient possible avec l'abeille anciennement sélectionné
  (if IsSelected
    _
    (else
      (Variables|Default|SetIsSelected? true)))
  (bind _outactors (Actor|GetAllActorsOfClass "/Game/Blueprints/Blueprints/Alveoles/BP_Alveole.BP_Alveole_C"))
  (Class|BPIAlveole|SetOutOfrange(Message) _outactors)
  (Audio|PlaySound2D "/Game/SFX/Sfx_Selected.Sfx_Selected" 1.0 1.0 0.0 0 0)
  (CallFunction|CheckSurroundings)
  (CallFunction|IsHighlighted? false))

(event EventMoveBeeto
  (params (AlveoleActor :type Actor%20Object%20Reference))
  ;[0.15 0.15 0.15 0.5] Gère le déplacement de l'abeille à l'endroit sélectionné
  ;;[0.15 0.15 0.15 0.5] Si l'abeille est sélectionné, elle peut-être joué
  (if (Variables|Default|GetIsSelected?)
    ;;[0.15 0.15 0.15 0.5] Déplace l'abeille à l'aveole correspondante
    (Transformation|SetActorLocation (+ (Transformation|GetActorLocation AlveoleActor) "0.000000,0.000000,10.000000") false false)
    (Utilities|SetsSpacesUnavailable
      (:Completed
        (Audio|PlaySound2D "/Game/SFX/Swish/Sfx_MoveSwish000.Sfx_MoveSwish000" 1.0 1.0 0.0 0 0)
        (CallFunction|CheckSurroundings)))))

(event EventDetectAvailableSpaces
  ;[0.15 0.15 0.15 0.5] Loop dans toute les alvéoles et les mets non disponible
  (bind (_currentalveole _accessible_ _freealveole) (Utilities|SetAvailableSpaces "/Game/Blueprints/Blueprints/Alveoles/BP_Alveole.BP_Alveole_C" (Math|Conversions|ToFloat(Integer) (Variables|Default|GetDistance%20Deplacement)))
    (:ForLoop
      (Class|BPIAlveole|AvailabilitySet(Message) _currentalveole _accessible_))
    (:Completed
      (Variables|Default|SetCurrentFreeSpaces _freealveole))))

(event EventBeginPlay
  (Class|BPIUIManager|GetHudRef(Message) (HUD|GetHUD (Game|GetPlayerController 0))))

(event EventIsHighlighted?
  (params (IsHighlighted :type Boolean))
  (bind _materiainstabeille (Variables|Materials|GetMateriaInstAbeille))
  (if IsHighlighted
    (Rendering|Material|SetVectorParameterValue _materiainstabeille "Tint" "(R=1.000000,G=0.075968,B=0.000000,A=1.000000)" :!class /Script/Engine.MaterialInstanceDynamic)
    (else
      (Rendering|Material|SetVectorParameterValue _materiainstabeille "Tint" "(R=1.000000,G=1.000000,B=1.000000,A=1.000000)" :!class /Script/Engine.MaterialInstanceDynamic))))

(fn ConstructionScript
  (bind _datatable (Variables|Default|GetDataTable))
  ;[0.15 0.15 0.15 0.5] Vérifie et stock les information de l'abeille sélectionné
  (bind _outrownames (DataTable|GetDataTableRowNames _datatable))
  (bind _returnvalue (Class|DataTableFunctionLibrary|DoesDataTableRowExist _datatable (Utilities|Array|Get(acopy) _outrownames (Math|Conversions|ToInteger(Byte) (Variables|01-SetupAlveole|GetTypeAbeille)))))
  (if _returnvalue
    (bind _returnvalue_2 (Utilities|GetDataTableRow _datatable (Utilities|Array|Get(acopy) _outrownames (Math|Conversions|ToInteger(Byte) (Variables|01-SetupAlveole|GetTypeAbeille))))
      (:then
        (Variables|Default|SetStructureAbeille _returnvalue_2)
        ;[0.15 0.15 0.15 0.5] Instance le materiel Master Instance d'alvéole
        (bind _returnvalue_3 (Rendering|Material|CreateDynamicMaterialInstance (Variables|Materials|GetMasterMaterialAbeille) "None" "None" :!class /Script/Engine.KismetMaterialLibrary))
        (Variables|Materials|SetMateriaInstAbeille _returnvalue_3)
        (CallFunction|ChangementTextureAbeille)
        (CallFunction|SetupInitial)))))

(fn ChangementTextureAbeille
  (bind _materiainstabeille (Variables|Materials|GetMateriaInstAbeille))
  (bind _structureabeille (Variables|Default|GetStructureAbeille))
  (bind _imageabeille (Utilities|Struct|BreakStruct_Abeille _structureabeille))
  ;[0.15 0.15 0.15 0.5] Applique la texture correspondante à l'alvéole choisi
  (Rendering|Material|SetTextureParameterValue _materiainstabeille "Diffuse" _imageabeille)
  (Rendering|Material|SetTextureParameterValue _materiainstabeille "OpacityMask" _imageabeille)
  ;[0.15 0.15 0.15 0.5] Applique le materiel après le changement de texture
  (Rendering|Material|SetMaterial (Variables|Default|GetAbeille) 0 (Variables|Materials|GetMateriaInstAbeille)))

(fn SetupInitial
  (bind _structureabeille (Variables|Default|GetStructureAbeille))
  (bind (_nom _typeabeille _pointdevie _distancedeplacement) (Utilities|Struct|BreakStruct_Abeille _structureabeille))
  (bind _output_get (Variables|Vie|SetVieMax _pointdevie))
  (Variables|Vie|SetVieActuelle _output_get)
  (Variables|Default|SetDistance%20Deplacement (* _distancedeplacement 256)))

(fn ActorProche
  (params (FiltreActor :type Object%20Class%20Reference) (SphereRadius :type Float%20%28single-precision%29))
  (bind _returnvalue (Transformation|GetActorLocation))
  ;[0.15 0.15 0.15 0.5] Effectue une zone des alveoles à porté selon  le type d'abeille
  ;;[0.15 0.15 0.15 0.5] Sphere debug spawn for actor detection
  (bind (_outactors _returnvalue_2) (Collision|SphereOverlapActors _returnvalue SphereRadius (Utilities|Array|MakeArray "ObjectTypeQuery1" "ObjectTypeQuery2") FiltreActor (Utilities|Array|MakeArray self)))
  ;;[0.15 0.1193 0 0.5] Debug position location
  (Rendering|Debug|DrawDebugSphere _returnvalue 1e+02 12 "(R=1.000000,G=0.020602,B=0.000000,A=1.000000)" 1e+01 5.0)
  (CallFunction|PrintMessage true "" (Utilities|GetDisplayName (Utilities|Array|Get(acopy) _outactors)) "(R=1.000000,G=0.515661,B=0.000000,A=1.000000)" 1e+01)
  (return _outactors _returnvalue_2))

(fn CanAttack?
  (bind _actordetecte (CallFunction|ActorProche "BP_Abeille_Parent_C" 0.0))
  (return _actordetecte))

(fn CanPond?
  (return false))

(fn GetAbeilleInfos
  (return (Variables|Default|GetStructureAbeille)))

(fn GetAlveoleInfos
  (bind _returnvalue (Transformation|GetActorLocation))
  (bind _outhit (Collision|LineTraceByChannel _returnvalue (- _returnvalue "0.000000,0.000000,100.000000") "TraceTypeQuery1" false 0 "None"))
  (bind _typealveole (Class|BPIAlveole|AlveoleType(Message) (.HitActor (Collision|BreakHitResult _outhit))))
  (CallFunction|PrintMessage true "BP_Abeille:: Get alveoleType ::" (Utilities|String|Append (Utilities|GetDisplayName (.HitActor (Collision|BreakHitResult _outhit))) "   " (Utilities|String|EnumtoString _typealveole)) "(R=0.435341,G=0.000000,B=1.000000,A=1.000000)" 5.0)
  (return _typealveole))

(fn GetBeeType
  (return (Variables|01-SetupAlveole|GetTypeAbeille)))

(fn GetSurroundingBees
  (return (Variables|Default|GetCurrentAttackableActors)))

(fn IsSpaceReacheable?
  (params (ActorToCheck :type Actor%20Object%20Reference))
  (return (Utilities|Array|ContainsItem (Variables|Default|GetCurrentFreeSpaces) ActorToCheck)))