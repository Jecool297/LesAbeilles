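; Queen bee child Blueprint (Abeille Reine) that tracks whether the queen can lay eggs to make a troop.
; CheckSurroundings sets CanMakeTroop by comparing the honeycomb cell (alvéole) info to one enum value, then prints a debug message.
; It then passes the flag to the custom HUD's troop message, while CanPond exposes it as a getter.
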(event EventBeginPlay
  (|CallParentFunction) ; This node is disabled and will not be called.\nDrag off pins to build functionality.
)

(event Collision|EventActorBeginOverlap
  (params (OtherActor :type Actor%20Object%20Reference)))

(event EventTick
  (params (DeltaSeconds :type Float%20%28single-precision%29)))

(event EventCheckSurroundings
  (bind _infosalveole (CallFunction|GetAlveoleInfos))
  (bind _output_get (Variables|Default|SetCanMakeTroop (Utilities|Enum|Equal(Enum) _infosalveole "NewEnumerator3")))
  (CallFunction|PrintMessage true "BP_ChildAbeille_Reine ::  Can make kids" " Is making a troop" "(R=0.164991,G=1.000000,B=0.000000,A=1.000000)" 1e+01)
  (bind _asbp_custom_hud (Utilities|Casting|CastToBP_CustomHUD (HUD|GetHUD (Game|GetPlayerController 0))))
  (Class|BPIUIManager|CanMakeTroop?(Message) (Variables|/Game/Blueprints/GameMode/BP_CustomHUD.BP_CustomHUD_C|GetHud _asbp_custom_hud) _output_get))

(fn ConstructionScript
  (|CallParentFunction))

(fn CanPond?
  (return (Variables|Default|GetCanMakeTroop)))