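; Soldier bee child Blueprint that detects enemy bees it can attack.
; CheckSurroundings un-highlights and clears previous targets, then searches a sphere sized by its movement distance for bees tagged RedTeam.
; It sends the resulting list and a can-attack flag to the player's HUD through interface messages.
; GetSurroundingBees exposes the current target list.
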(event EventBeginPlay
  (|CallParentFunction) ; This node is disabled and will not be called.\nDrag off pins to build functionality.
)

(event Collision|EventActorBeginOverlap
  (params (OtherActor :type Actor%20Object%20Reference)))

(event EventCheckSurroundings
  (bind _currentattackableactors (Variables|Default|GetCurrentAttackableActors))
  (bind _currentattackableactors_2 (Variables|Default|GetCurrentAttackableActors))
  (for _array_element _currentattackableactors
    (Class|BPI|IsHighlighted?(Message) _array_element false))
  (Utilities|Array|Clear _currentattackableactors)
  (bind (_actordanslazone _actordetecte) (CallFunction|ActorProche "/Game/Blueprints/Blueprints/Abeilles/BP_Abeille_Parent.BP_Abeille_Parent_C" (Math|Conversions|ToFloat(Integer) (Variables|Default|GetDistance%20Deplacement))))
  (for _array_element_2 _actordanslazone
    (if (and (Actor|ActorHasTag _array_element_2 "RedTeam") _actordetecte)
      (Utilities|Array|AddUnique (Variables|Default|GetCurrentAttackableActors) _array_element_2)))
  (Class|BPIUIManager|CanAttack?(Message) (HUD|GetHUD (Game|GetPlayerController 0)) (Utilities|Array|IsNotEmpty _currentattackableactors_2) _currentattackableactors_2))

(fn ConstructionScript
  (|CallParentFunction))

(fn GetSurroundingBees
  (return (Variables|Default|GetCurrentAttackableActors)))