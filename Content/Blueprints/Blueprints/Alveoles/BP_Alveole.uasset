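; BP_Alveole is a selectable honeycomb cell with a type-specific texture and a tint showing whether it is occupied.
; The construction script creates a dynamic material instance and sets its diffuse texture from TypeAlveole.
; AvalabilityCheck traces upward, ignoring other cells, and returns the raw hit, so IsAvailable is true when something blocks the cell.
; AvailabilitySet tints red for true and green for false, while SetOutOfrange resets to white.
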(event EventSetOutOfrange
  (bind _materiainstalveole (Variables|Materials|GetMateriaInstAlveole))
  ;[0.15 0.15 0.15 0.5] Si l'alveole est libre, la couleur verte est mise et la case est coché comme disponible
  (Rendering|Material|SetScalarParameterValue _materiainstalveole "EmissiveIntensity" 0.0 :!class /Script/Engine.MaterialInstanceDynamic)
  (Rendering|Material|SetVectorParameterValue _materiainstalveole "Tint" "(R=1.000000,G=1.000000,B=1.000000,A=1.000000)" :!class /Script/Engine.MaterialInstanceDynamic))

(event EventAvailabilitySet
  (params (SpaceAvailable? :type Boolean))
  (bind _returnvalue (Math|Float|SelectFloat 0.0 0.0 SpaceAvailable?))
  (bind _materiainstalveole (Variables|Materials|GetMateriaInstAlveole))
  ;[0.15 0.15 0.15 0.5] Change la couleur de l'aveole selon si elle est occupé ou non
  (if SpaceAvailable?
    ;;[0.15 0.15 0.15 0.5] Si l'alveole est occupé, la couleur rouge est mise et la case est coché comme indisponible
    (Rendering|Material|SetScalarParameterValue (Variables|Materials|GetMateriaInstAlveole) "EmissiveIntensity" _returnvalue :!class /Script/Engine.MaterialInstanceDynamic)
    (Rendering|Material|SetVectorParameterValue _materiainstalveole "Tint" "(R=0.479167,G=0.000000,B=0.005480,A=1.000000)" :!class /Script/Engine.MaterialInstanceDynamic)
    (else
      ;;[0.15 0.15 0.15 0.5] Si l'alveole est libre, la couleur verte est mise et la case est coché comme disponible
      (Rendering|Material|SetScalarParameterValue _materiainstalveole "EmissiveIntensity" _returnvalue :!class /Script/Engine.MaterialInstanceDynamic)
      (Rendering|Material|SetVectorParameterValue _materiainstalveole "Tint" "(R=0.073602,G=1.000000,B=0.001521,A=1.000000)" :!class /Script/Engine.MaterialInstanceDynamic))))

(fn ConstructionScript
  ;[0.15 0.15 0.15 0.5] Instance le materiel Master Instance d'alvéole
  (bind _returnvalue (Rendering|Material|CreateDynamicMaterialInstance (Variables|Materials|GetMasterMaterialAlveole) "None" "None" :!class /Script/Engine.KismetMaterialLibrary))
  (Variables|Materials|SetMateriaInstAlveole _returnvalue)
  (CallFunction|ChangementTextureAlveole))

(fn ChangementTextureAlveole
  ;[0.15 0.15 0.15 0.5] Applique la texture correspondante à l'alvéole choisi
  (Rendering|Material|SetTextureParameterValue (Variables|Materials|GetMateriaInstAlveole) "Diffuse" (Utilities|Array|Get(acopy) (Variables|Materials|GetAlveoleTexture) (Math|Conversions|ToInteger(Byte) (Variables|01-SetupAlveole|GetTypeAlveole))))
  ;[0.15 0.15 0.15 0.5] Applique le materiel après le changement de texture
  (Rendering|Material|SetMaterial (Variables|Default|GetAlveole) 0 (Variables|Materials|GetMateriaInstAlveole)))

(fn AlveoleType
  (return (Variables|01-SetupAlveole|GetTypeAlveole)))

(fn AvalabilityCheck
  (bind _returnvalue (Transformation|GetActorLocation))
  ;[0.15 0.15 0.15 0.5] Regarde Qu'aucune abeille ou autre acteur n'est sur l'alveole qui tente d'être sélectionné
  (bind _outactors (Actor|GetAllActorsOfClass "BP_Alveole_C"))
  (bind _returnvalue_2 (Collision|LineTraceByChannel (+ _returnvalue "0.000000,0.000000,10.000000") (+ _returnvalue "0.000000,0.000000,100.000000") "TraceTypeQuery1" false _outactors "ForDuration"))
  (bind _output_get (Variables|Default|SetIsAvailable? _returnvalue_2))
  (return _output_get))