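; BP_PlateauSpawner builds the game board ("plateau") as a staggered honeycomb grid of BP_Alveole cells when play begins.
; It measures cell size from a temporary static mesh component, then spawns NbrVerticale by NbrHorizontale cells, offsetting odd rows and randomizing each TypeAlveole.
; A separate CreationAlveole function, unused by BeginPlay, spawns and attaches one cell, records its type and computes the next position via ProchainePositionAlveole.
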(event EventBeginPlay
  (bind _returnvalue (AddComponent|AddStaticMeshComponent false))
  (Variables|AlveoleRelated|SetDimensionsAlveole (* (.BoxExtent (Collision|GetComponentBounds _returnvalue)) 2.0))
  (Components|DestroyComponent _returnvalue)
  (for _index (range 0 (- (Variables|GenerationPlateau|GetNbrVerticale) 1))
    (for _index_2 (range 0 (- (Variables|GenerationPlateau|GetNbrHorizontale) 1))
      (Game|SpawnActorfromClass "/Game/Blueprints/Blueprints/Alveoles/BP_Alveole.BP_Alveole_C" (Math|Transform|MakeTransform (Math|Vector|MakeVector (* _index (* (.Y (Math|Vector|BreakVector (Variables|AlveoleRelated|GetDimensionsAlveole))) 0.8)) (+ (* (.Y (Math|Vector|BreakVector (Variables|AlveoleRelated|GetDimensionsAlveole))) _index_2) (Math|Float|SelectFloat 0.0 (* (.X (Math|Vector|BreakVector (Variables|AlveoleRelated|GetDimensionsAlveole))) 0.6) (== (Math|Integer|%(Integer) _index 2) 0))) 0.0) "0, 0, 0" "1.000000,1.000000,1.000000") "Undefined" "MultiplyWithRoot" 0 (Utilities|Select :Index (Math|Random|RandomIntegerinRange 0 3) :Option%200 "NewEnumerator1" :Option%201 "NewEnumerator0" :Option%202 "NewEnumerator2" :Option%203 "NewEnumerator3") 0))))

(fn ConstructionScript)

(fn CreationAlveole
  (params (Position%20Spawn%20Alveole :type Vector) (Type%20Alveole :type Enum_TypeAlveole%20Enum :default "NewEnumerator0"))
  ;[0.15 0.15 0.15 0.5] Fait apparaitre une parcel (Alveole) et l'ajoute à la liste de parcel joint à son type d'alveole
  (bind _returnvalue (Game|SpawnActorfromClass "/Game/Blueprints/Blueprints/Alveoles/BP_Alveole.BP_Alveole_C" (Math|Transform|MakeTransform Position%20Spawn%20Alveole "0, 0, 0" "1.000000,1.000000,1.000000") "AlwaysSpawn" "OverrideRootScale" self Type%20Alveole 0))
  (Utilities|Map|Add (Variables|AlveoleRelated|GetListAlveolePlateau) _returnvalue (Variables|/Game/Blueprints/Blueprints/Alveoles/BP_Alveole.BP_Alveole_C|GetTypeAlveole _returnvalue))
  ;;[0.15 0.15 0.15 0.5] Attache l'alveole au plateau
  (Transformation|AttachActorToActor _returnvalue self "None" "KeepRelative" "KeepRelative" "KeepRelative" false)
  ;;[0.15 0.15 0.15 0.5] Récupère les dimensions de l'aveole qui viens d'apparaitre et calcule la prochaine position d'apparition
  (Utilities|ProchainePositionAlveole _returnvalue)
  (return))