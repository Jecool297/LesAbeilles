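; BP_CustomHUD creates and owns the game's WBP_HUD widget.
; On BeginPlay it builds the widget for the first player, collapses its actions message, adds it to the player screen and sets Game and UI input mode.
; It forwards attack availability and attackable bees to the widget through a CanAttack? event, and exposes the widget through GetHudRef.
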(event EventBeginPlay
  ;[0.15 0.15 0.15 0.5] Creates the HUD and stores it
  (bind _returnvalue (UserInterface|CreateWidget "/Game/Widget/HUD/WBP_HUD.WBP_HUD_C" (Game|GetPlayerController 0)))
  (bind _output_get (Variables|Default|SetHud _returnvalue))
  (Class|BPIUIManager|HideActions(Message) _output_get "Collapsed")
  ;[0.15 0.15 0.15 0.5] Adds the HUD to the player's screen while enabling UI input mode
  (UserInterface|Viewport|AddtoPlayerScreen _output_get)
  (Input|SetInputModeGameandUI (Game|GetPlayerController 0) 0 "DoNotLock" false false))

(event EventCanAttack?
  (params (CanAttack? :type Boolean) (AttackableBees :type Array%20of%20Actor%20Object%20References))
  (Default|CanAttack? (Variables|Default|GetHud) CanAttack? AttackableBees))

(fn ConstructionScript)

(fn GetHudRef
  (return (Variables|Default|GetHud)))