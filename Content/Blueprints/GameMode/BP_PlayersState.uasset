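; Player state for a turn-based game that tracks whether its player has played the current turn.
; TourCompleter sets the TourJouee flag, prints a debug message and asks GS_GameGlobalState to run CheckTurn.
; TourReset clears the flag, and TurnCheck returns it.
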(event Custom|TourReset
  (Variables|Default|SetTourJouee false))

(event EventBeginPlay
  (Development|PrintString "Player State Initialise"))

(event EventTick
  (params (DeltaSeconds :type Float%20%28single-precision%29)))

(event EventTourCompleter
  (CallFunction|PrintMessage true "Game State : Played Turn" "Turn Played " "(R=0.293710,G=1.000000,B=0.000000,A=1.000000)" 5.0)
  (Variables|Default|SetTourJouee true)
  (bind _asgs_game_global_state (Utilities|Casting|CastToGS_GameGlobalState (Game|GetGameState)))
  (Default|CheckTurn _asgs_game_global_state))

(fn ConstructionScript)

(fn TurnCheck
  (return (Variables|Default|GetTourJouee)))