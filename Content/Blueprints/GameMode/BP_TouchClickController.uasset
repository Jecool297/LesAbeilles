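; Player controller that turns touch input into a world click location for BP_SpriteTest.
; On BeginPlay it adds the IMC_Mobile Enhanced Input mapping and enables Game and UI input with a visible cursor.
; When IA_Touch starts, it traces under the cursor on the Visibility channel and passes the hit location to the first BP_SpriteTest found, without checking for a hit.
; Screen-to-world deprojection nodes are left unused.
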(event Input|EnhancedActionEvents|EnhancedInputActionIA_Touch
  (params (ActionValue :type Boolean) (ElapsedSeconds :type Float%20%28double-precision%29) (TriggeredSeconds :type Float%20%28double-precision%29) (InputAction :type Input%20Action%20Object%20Reference :default "/Game/Controls/IA_Touch.IA_Touch"))
  (:Started
    (bind _returnvalue (Actor|GetActorOfClass "/Game/Art/Personnages/FlipBook/BP_SpriteTest.BP_SpriteTest_C"))
    (Default|ClickLocation _returnvalue (.Location (Collision|BreakHitResult (.HitResult (Game|Player|GetHitResultUnderCursorbyChannel "TraceTypeQuery1" true)))))))

(event EventBeginPlay
  (bind _returnvalue (PlayerController|LocalPlayerSubsystems|GetEnhancedInputLocalPlayerSubsystem))
  (Utilities|IsValid _returnvalue
    (:Is%20Valid
      (Input|AddMappingContext _returnvalue "/Game/Controls/IMC_Mobile.IMC_Mobile" 0 "(bIgnoreAllPressedKeysUntilRelease=True,bForceImmediately=False,bNotifyUserSettings=False)")
      (Input|SetInputModeGameandUI (Game|GetPlayerController 0) 0 "DoNotLock" false false)
      (Variables|/Script/Engine.PlayerController|SetbShowMouseCursor (Game|GetPlayerController 0) true))))

(fn ConstructionScript)