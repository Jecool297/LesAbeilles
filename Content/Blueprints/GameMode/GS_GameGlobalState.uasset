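; Game state for a two-player turn-based game that tracks which player's turn it is.
; CheckTurn flips CurrentTurnIndex between 0 and 1 on the authority.
; The OnRep_CurrentIndex event calls SetTurn on the current player's BP_TouchClickController, true only if that player is the first local player.
; The OnRep_CurrentTurnIndex function is empty, and nothing here calls that event.
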(event Custom|OnRep_CurrentIndex
  (Variables|Default|SetPlayer%20State (Variables|/Script/Engine.Controller|GetPlayerState (Game|GetPlayerController 0)))
  (bind _output_get (Variables|Default|SetCurrentPlayerTurn (Utilities|Array|Get(acopy) (Variables|Default|GetPlayerArray) (Variables|Default|GetCurrentTurnIndex))))
  (if (== _output_get (Variables|Default|GetPlayer%20State))
    (bind _asbp_touch_click_controller (Utilities|Casting|CastToBP_TouchClickController (Game|GetPlayerController (Variables|Default|GetCurrentPlayerTurn))))
    (Default|SetTurn _asbp_touch_click_controller true)
    (else
      (bind _asbp_touch_click_controller_2 (Utilities|Casting|CastToBP_TouchClickController (Game|GetPlayerController (Variables|Default|GetCurrentPlayerTurn))))
      (Default|SetTurn _asbp_touch_click_controller_2 false))))

(event EventBeginPlay)

(event EventTick
  (params (DeltaSeconds :type Float%20%28single-precision%29)))

(fn ConstructionScript)

(fn CheckTurn
  (Networking|SwitchHasAuthority
    (:Authority
      (Development|PrintString "Has Authority")
      (Variables|Default|SetCurrentTurnIndex (- 1 (Variables|Default|GetCurrentTurnIndex)))
      (return))
    (:Remote
      (Development|PrintString "Has Authority"))))

(fn OnRepCurrentTurnIndex)